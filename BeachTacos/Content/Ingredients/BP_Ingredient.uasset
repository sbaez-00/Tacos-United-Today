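; BP_Ingredient is an ingredient actor whose look, name and identifier come from its DAIngredientConstruction data.
; The construction script blocking-loads the mesh and applies a dynamic instance of M_PH_Ingredient tinted with the data's color.
; On BeginPlay it copies the ingredient name to the interaction component as its owner name.
; GetIngredientIdentifier exposes the identifier and name to callers.
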(event EventBeginPlay
  (CallFunction|SetupInteraction))

(event Collision|EventActorBeginOverlap
  (params (OtherActor :type Actor%20Object%20Reference)))

(event EventTick
  (params (DeltaSeconds :type Float%20%28single-precision%29)))

(fn ConstructionScript
  (bind _mesh (Variables|Default|GetMesh))
  (bind _da_ingredientconstruction (Variables|Default|GetDA_IngredientConstruction))
  (bind _returnvalue (Utilities|LoadAssetBlocking (Variables|/Game/Ingredients/PDA_IngredientBase.PDA_IngredientBase_C|GetMesh _da_ingredientconstruction)))
  (bind _asstatic_mesh (Utilities|Casting|CastToStaticMesh _returnvalue))
  (Components|StaticMesh|SetStaticMesh _mesh _asstatic_mesh)
  (bind _returnvalue_2 (Rendering|Material|CreateDynamicMaterialInstance _mesh 0 "/Game/PlaceholderMaterials/M_PH_Ingredient.M_PH_Ingredient" "" :!class /Script/Engine.PrimitiveComponent))
  (Rendering|Material|SetVectorParameterValue _returnvalue_2 "Color" (Variables|/Game/Ingredients/PDA_IngredientBase.PDA_IngredientBase_C|GetColor _da_ingredientconstruction) :!class /Script/Engine.MaterialInstanceDynamic))

(fn SetupInteraction
  (Variables|/Game/BPC_InteractionComponent.BPC_InteractionComponent_C|SetOwner%20Name (Variables|Default|GetBPC_InteractionComponent) (Variables|/Game/Ingredients/PDA_IngredientBase.PDA_IngredientBase_C|GetName (Variables|Default|GetDA_IngredientConstruction))))

(fn GetIngredientIdentifier
  (bind _da_ingredientconstruction (Variables|Default|GetDA_IngredientConstruction))
  (return (Variables|/Game/Ingredients/PDA_IngredientBase.PDA_IngredientBase_C|GetIndentifier _da_ingredientconstruction) (Variables|/Game/Ingredients/PDA_IngredientBase.PDA_IngredientBase_C|GetName _da_ingredientconstruction)))